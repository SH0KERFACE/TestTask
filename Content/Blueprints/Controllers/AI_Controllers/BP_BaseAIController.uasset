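; Base AI controller that sends its BP_BaseAIChar pawn to that character's TargetActor on BeginPlay.
; The GoToTarget macro wraps AI MoveTo with finished, failed and invalid-actor exits.
; Whether the move finishes or fails, PrintItems prints each item ID and count from the character's inventory component as debug text.
; Setup runs once on BeginPlay rather than on possess, and stops if the controlled pawn cast fails.
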(event `self.ReceiveBeginPlay`
  (bind _asbp_base_aichar (cast `/Game/Blueprints/Characters/BP_BaseAIChar` (`self.K2_GetPawn`)))
  (bind _output_get (set `self.As BP Base AIChar` _asbp_base_aichar))
  (`/Engine/EditorBlueprintResources/StandardMacros.IsValid` (`/Game/Blueprints/Characters/BP_BaseAIChar.TargetActor` _output_get)
    (:`Is Valid`
      (`self.GoToTarget` _output_get
        (:`On Request Finished`
          (`self.PrintItems` (`/Game/Blueprints/Characters/BP_BaseAIChar.BP_InventoryComp` _output_get) :!label _label))
        (:`On Request Failed`
          (goto _label))
        (:`Actor Not Valid`
          (`KismetSystemLibrary.PrintString` "Not valid target actor"))))))

(fn `PrintItems`
  (params (InventoryComp :type "/Game/Blueprints/Components/BP_InventoryComp Object Reference"))
  (bind _inventory (`/Game/Blueprints/Components/BP_InventoryComp.Inventory` InventoryComp))
  (`/Engine/EditorBlueprintResources/StandardMacros.IsValid` InventoryComp
    (:`Is Valid`
      (bind _keys (`BlueprintMapLibrary.Map_Keys` _inventory))
      (for _array_element _keys
        (bind (_value _returnvalue) (`BlueprintMapLibrary.Map_Find` _inventory _array_element))
        (if _returnvalue
          (`KismetSystemLibrary.PrintString` (`KismetStringLibrary.Concat_StrStr` "ItemId: " (`KismetStringLibrary.Conv_IntToString` _array_element) "//Count: " (`KismetStringLibrary.Conv_IntToString` _value)) true true (struct :`G` 0.66 :`B` 1.0 :`A` 1.0) 15.0))))))

(fn `UserConstructionScript`)