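; Base item actor that configures itself from the DTItems data table and is destroyed when interacted with.
; The construction script searches the table rows for a unique ID matching ItemID, then copies the row's struct and name and applies its static mesh and scale, printing a warning if the mesh is invalid.
; InteractItem only destroys the actor, while GetItemInfo exposes the ItemID.
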(event `/Game/Blueprints/Interfaces/BPI_InteractableItem.InteractItem`
  (`self.K2_DestroyActor`))

(fn `GetItemInfo`
  (returns (UniqueID :type Integer))
  (return (`self.ItemID`)))

(fn `UserConstructionScript`
  (locals (DT_Items :type "DataTable Object Reference" :default "/Script/Engine.DataTable'/Game/Blueprints/Structs/DT_Item.DT_Item'") (ItemSctruct :type "/Game/Blueprints/Structs/ItemStruct Structure"))
  (bind _dt_items (`local.DT_Items`))
  (bind _outrownames (`DataTableFunctionLibrary.GetDataTableRowNames` _dt_items))
  (for _array_element _outrownames
    (bind _returnvalue (`|GetDataTableRow` _dt_items _array_element)
      (:`then`
        (bind _returnvalue_2 (== (`self.ItemID`) (`.IemUniqueID_4_029F1EB3418423CF3CEED6BDA4BF83A0` (break `/Game/Blueprints/Structs/ItemStruct` _returnvalue))))
        (if _returnvalue_2
          (break)))))
  (if _returnvalue_2
    (bind _output_get (set `local.ItemSctruct` _returnvalue))
    (set `self.ItemName` (`.ItemName_5_23FF66BE45BD5E138A07218B8FDA1CF1` (break `/Game/Blueprints/Structs/ItemStruct` _output_get)))
    (`/Engine/EditorBlueprintResources/StandardMacros.IsValid` (`.StaticMesh_8_5FF5236B4C6202D908E2C98D9A7BFFAE` (break `/Game/Blueprints/Structs/ItemStruct` _output_get))
      (:`Is Valid`
        (`StaticMeshComponent.SetStaticMesh` (`self.StaticMesh`) (`.StaticMesh_8_5FF5236B4C6202D908E2C98D9A7BFFAE` (break `/Game/Blueprints/Structs/ItemStruct` _output_get)))
        (`SceneComponent.SetRelativeScale3D` (`self.StaticMesh`) (`.ItemScale_11_1F15652646ED3B68DD63DB9B0E33BDE1` (break `/Game/Blueprints/Structs/ItemStruct` (`local.ItemSctruct`)))))
      (:`Is Not Valid`
        (`KismetSystemLibrary.PrintString` "StaticMesh not valid")))))